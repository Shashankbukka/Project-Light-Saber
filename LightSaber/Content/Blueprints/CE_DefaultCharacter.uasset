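; Player character wielding a lightsaber, with montage attacks, a randomized blade color, a held-space force jump and an options HUD toggle.
; A timeline extends and retracts the blade and toggles its light.
; While out, a per-tick sphere trace along the blade applies damage and buffers hits.
; Buffered hits become attached, fading burn decals with sparks, with midpoints interpolated between distant hits to fill gaps.
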(event EventBeginPlay
  (bind _asce_hud (Utilities|Casting|CastToCE_HUD (HUD|GetHUD (Game|GetPlayerController 0))))
  (Variables|Default|SetHUDRef _asce_hud)
  (switch int (Math|Random|RandomIntegerinRange 0 4)
    (:0
      (Variables|Default|SetColor "(R=30.000000,G=1.000000,B=1.000000,A=1.000000)"))
    (:1
      (Variables|Default|SetColor "(R=1.000000,G=30.000000,B=1.000000,A=1.000000)"))
    (:2
      (Variables|Default|SetColor "(R=1.000000,G=1.000000,B=30.000000,A=1.000000)"))
    (:3
      (Variables|Default|SetColor "(R=20.000000,G=1.000001,B=15.000000,A=1.000000)"))
    (:4
      (Variables|Default|SetColor "(R=15.000000,G=13.000000,B=1.000001,A=1.000000)")))
  (Rendering|Material|SetVectorParameterValue (Variables|Default|GetSaberMat) "Color" (Variables|Default|GetColor) :!class /Script/Engine.MaterialInstanceDynamic)
  (bind _output_get (Variables|Default|SetColor (Math|Color|MakeColor (/ (.R (Math|Color|BreakColor (Variables|Default|GetColor))) 1e+01) (/ (.G (Math|Color|BreakColor (Variables|Default|GetColor))) 1e+01) (/ (.B (Math|Color|BreakColor (Variables|Default|GetColor))) 1e+01) (.A (Math|Color|BreakColor (Variables|Default|GetColor))))))
  (Effects|Components|ParticleSystem|SetColorParameter (Variables|Default|GetParticleSystem) "Color" _output_get)
  (Rendering|Components|Light|SetLightColor (Variables|Default|GetPointLight) (Variables|Default|GetColor) true))

(event EventTick
  (params (DeltaSeconds :type Float%20%28single-precision%29))
  (bind _mesh (Variables|Character|GetMesh))
  (bind _structarray (Variables|Default|GetStructArray))
  (bind _vectorlocationsforsaberburnarray (Variables|Default|GetVectorLocationsForSaberBurnArray))
  (bind _returnvalue (Transformation|GetSocketLocation _mesh "111"))
  (bind _output (Utilities|Array|Get(acopy) _structarray 1))
  (bind _output_2 (Utilities|Array|Get(acopy) _structarray 2))
  (bind (_location _normal) (Utilities|Struct|BreakSaberDecalStruct _output))
  (bind (_location_2 _normal_2 _hitcomponent _hitbone) (Utilities|Struct|BreakSaberDecalStruct _output_2))
  (bind _returnvalue_2 (Math|Conversions|RotationFromXVector _normal))
  (bind _returnvalue_3 (- _location _location_2))
  (bind (_roll _pitch _yaw) (Math|Rotator|BreakRotator _returnvalue_2))
  (bind _returnvalue_4 (/ _returnvalue_3 2.0))
  (bind _returnvalue_5 (- _location _returnvalue_4))
  (bind _returnvalue_6 (- _location _returnvalue_5))
  (bind _returnvalue_7 (/ _returnvalue_6 2.0))
  (bind _returnvalue_8 (- _location _returnvalue_7))
  (bind _returnvalue_9 (- _returnvalue_5 _returnvalue_7))
  (bind _returnvalue_10 (- _location _returnvalue_8))
  (bind _returnvalue_11 (/ _returnvalue_10 2.0))
  (if (Variables|Default|Getissaberout)
    ;[1 1 1] Does a trace for the blade
    (bind (_outhit _returnvalue_12) (Collision|SphereTraceByChannel _returnvalue (+ _returnvalue (* (Math|Vector|GetForwardVector (Math|Rotator|FindLookatRotation _returnvalue (Transformation|GetSocketLocation _mesh "222"))) 1.1e+02)) 7.0 "TraceTypeQuery1" false 0 "None"))
    (if _returnvalue_12
      (Utilities|FlowControl|Sequence
        (:then_0
          (Utilities|Array|Add _structarray (Utilities|Struct|MakeSaberDecalStruct (.Location (Collision|BreakHitResult _outhit)) (.Normal (Collision|BreakHitResult _outhit)) (.HitComponent (Collision|BreakHitResult _outhit)) (.HitBoneName (Collision|BreakHitResult _outhit))))
          (if (> (Utilities|Array|Length _structarray) 3)
            ;[1 1 1] if distance between 2 points is more than X units, add additional points between them
            (if (> (Math|Vector|VectorLength _returnvalue_3) 4.0)
              ;[1 1 1] A messy mess of vector math for adding more points
              (Utilities|Array|Add _vectorlocationsforsaberburnarray _location)
              (Utilities|Array|Add _vectorlocationsforsaberburnarray _returnvalue_5)
              (Utilities|Array|Add _vectorlocationsforsaberburnarray _returnvalue_8)
              (Utilities|Array|Add _vectorlocationsforsaberburnarray _returnvalue_9)
              (Utilities|Array|Add _vectorlocationsforsaberburnarray (- _location _returnvalue_11))
              (Utilities|Array|Add _vectorlocationsforsaberburnarray (- _returnvalue_8 _returnvalue_11))
              (Utilities|Array|Add _vectorlocationsforsaberburnarray (- _returnvalue_9 _returnvalue_11))
              (Utilities|Array|Add _vectorlocationsforsaberburnarray (+ _returnvalue_9 _returnvalue_11))
              (else
                ;[1 1 1] if there's no need for extra points, just do the one
                (Utilities|Array|Add _vectorlocationsforsaberburnarray _location)))
            ;[1 1 1] dynamic material instance for every decal so fade out times are independent of each other
            (bind _returnvalue_13 (Rendering|Material|CreateDynamicMaterialInstance "/Game/Blueprints/burnmarks.burnmarks" :!class /Script/Engine.KismetMaterialLibrary))
            ;[1 1 1] spawns decals
            (for _array_element (Variables|Default|GetVectorLocationsForSaberBurnArray)
              (Class|GameplayStatics|SpawnDecalAttached _returnvalue_13 "12.000000,12.000000,12.000000" _hitcomponent _hitbone _array_element (Math|Rotator|MakeRotator _roll _pitch _yaw) "KeepWorldPosition" 15.0)
              ;[1 1 1] set spawn time for fading out effects in the material
              (Rendering|Material|SetScalarParameterValue _returnvalue_13 "SpawnTime" (Utilities|Time|GetGameTimeinSeconds) :!class /Script/Engine.MaterialInstanceDynamic))
            ;[1 1 1] removes oldest hit location from struct array  and clears all vector points
            (Utilities|Array|RemoveIndex _structarray)
            (Utilities|Array|Clear (Variables|Default|GetVectorLocationsForSaberBurnArray))
            ;[1 1 1] spawns particles from burned areas once every X seconds
            (Utilities|FlowControl|DoOnce false :!label _label
              (:Completed
                (Effects|SpawnEmitteratLocation "/Game/Blueprints/sparks.sparks" _location)
                (Utilities|FlowControl|Delay 0.03)
                (goto _label Reset)))))
        (:then_1
          ;[1 1 1] deals damage to things it hits
          (Game|Damage|ApplyDamage (.HitActor (Collision|BreakHitResult _outhit)) 3.0 0 0)))
      (else
        (Utilities|Array|Clear _structarray)))))

(event Input|AxisEvents|InputAxisMoveForward
  (params (AxisValue :type Float%20%28single-precision%29))
  ;[1 1 1] Inputs
  (Pawn|Input|AddMovementInput (Transformation|GetActorForwardVector) AxisValue false))

(event Input|AxisEvents|InputAxisMoveRight
  (params (AxisValue :type Float%20%28single-precision%29))
  ;[1 1 1] Inputs
  (Pawn|Input|AddMovementInput (Transformation|GetActorRightVector) AxisValue false))

(event Input|AxisEvents|InputAxisLookUp
  (params (AxisValue :type Float%20%28single-precision%29))
  ;[1 1 1] Inputs
  (Pawn|Input|AddControllerPitchInput (* AxisValue (Variables|Default|GetMouseAxisValueMultiplier))))

(event Input|AxisEvents|InputAxisLookRight
  (params (AxisValue :type Float%20%28single-precision%29))
  ;[1 1 1] Inputs
  (Pawn|Input|AddControllerYawInput (* (Variables|Default|GetMouseAxisValueMultiplier) AxisValue)))

(event Input|KeyboardEvents|0
  (params (Key :type Key%20Structure))
  (:Pressed
    (Development|ExecuteConsoleCommand "stat fps")))

(event Input|KeyboardEvents|9
  (params (Key :type Key%20Structure))
  (bind _hudref (Variables|Default|GetHUDRef))
  (:Pressed
    (Utilities|FlowControl|FlipFlop
      (:A
        (Default|ShowOptions _hudref)
        (Variables|/Script/Engine.PlayerController|SetbShowMouseCursor (Game|GetPlayerController 0) true)
        (CallFunction|DisableMouseLook))
      (:B
        (Default|HideOptions _hudref)
        (Variables|/Script/Engine.PlayerController|SetbShowMouseCursor (Game|GetPlayerController 0) false)
        (CallFunction|EnableMouseLook)))))

(event Input|MouseEvents|AltLeftMouseButton
  (params (Key :type Key%20Structure))
  (bind _particlesystem (Variables|Default|GetParticleSystem))
  (:Pressed
    (if (Variables|Default|Getreadytoattack)
      (Animation|PlayAnimMontage self "/Game/Assets/RK_combat_slash_Montage.RK_combat_slash_Montage" 1.0 "None")
      (Variables|Default|Setreadytoattack false)
      (if (Variables|Default|Getissaberout)
        (Effects|Particles|Trails|BeginTrails _particlesystem "111" "222" "ETrailWidthMode_FromCentre" 1.0))
      (Utilities|FlowControl|Delay 1.0)
      (Variables|Default|Setreadytoattack true)
      (Effects|Particles|Trails|EndTrails _particlesystem))))

(event Input|MouseEvents|CtrlLeftMouseButton
  (params (Key :type Key%20Structure))
  (bind _particlesystem (Variables|Default|GetParticleSystem))
  (:Pressed
    (if (Variables|Default|Getreadytoattack)
      (Animation|PlayAnimMontage self "/Game/Assets/RK_combat_thrust_Montage.RK_combat_thrust_Montage" 1.0 "None")
      (Variables|Default|Setreadytoattack false)
      (if (Variables|Default|Getissaberout)
        (Effects|Particles|Trails|BeginTrails _particlesystem "111" "222" "ETrailWidthMode_FromCentre" 1.0))
      (Utilities|FlowControl|Delay 1.0)
      (Variables|Default|Setreadytoattack true)
      (Effects|Particles|Trails|EndTrails _particlesystem))))

(event Input|MouseEvents|ShiftLeftMouseButton
  (params (Key :type Key%20Structure))
  (bind _particlesystem (Variables|Default|GetParticleSystem))
  (:Pressed
    (if (Variables|Default|Getreadytoattack)
      (Animation|PlayAnimMontage self "/Game/Assets/RK_swing_down_Montage.RK_swing_down_Montage" 1.0 "None")
      (Variables|Default|Setreadytoattack false)
      (if (Variables|Default|Getissaberout)
        (Effects|Particles|Trails|BeginTrails _particlesystem "111" "222" "ETrailWidthMode_FromCentre" 1.0))
      (Utilities|FlowControl|Delay 1.0)
      (Variables|Default|Setreadytoattack true)
      (Effects|Particles|Trails|EndTrails _particlesystem))))

(event Input|KeyboardEvents|2
  (params (Key :type Key%20Structure))
  (:Pressed
    (switch int (Math|Random|RandomIntegerinRange 0 4)
      (:0
        (Variables|Default|SetColor "(R=30.000000,G=1.000000,B=1.000000,A=1.000000)"))
      (:1
        (Variables|Default|SetColor "(R=1.000000,G=30.000000,B=1.000000,A=1.000000)"))
      (:2
        (Variables|Default|SetColor "(R=1.000000,G=1.000000,B=30.000000,A=1.000000)"))
      (:3
        (Variables|Default|SetColor "(R=20.000000,G=1.000001,B=15.000000,A=1.000000)"))
      (:4
        (Variables|Default|SetColor "(R=15.000000,G=13.000000,B=1.000001,A=1.000000)")))
    (Rendering|Material|SetVectorParameterValue (Variables|Default|GetSaberMat) "Color" (Variables|Default|GetColor) :!class /Script/Engine.MaterialInstanceDynamic)
    (bind _output_get (Variables|Default|SetColor (Math|Color|MakeColor (/ (.R (Math|Color|BreakColor (Variables|Default|GetColor))) 1e+01) (/ (.G (Math|Color|BreakColor (Variables|Default|GetColor))) 1e+01) (/ (.B (Math|Color|BreakColor (Variables|Default|GetColor))) 1e+01) (.A (Math|Color|BreakColor (Variables|Default|GetColor))))))
    (Effects|Components|ParticleSystem|SetColorParameter (Variables|Default|GetParticleSystem) "Color" _output_get)
    (Rendering|Components|Light|SetLightColor (Variables|Default|GetPointLight) (Variables|Default|GetColor) true)))

(event Input|KeyboardEvents|1
  (params (Key :type Key%20Structure))
  (bind _saberblade (Variables|Default|Getsaberblade))
  (:Pressed
    (Utilities|FlowControl|Sequence
      (:then_0
        (Utilities|FlowControl|FlipFlop
          (:A
            (Variables|Default|Setisforwarding true)
            (bind (_direction _size _location) (Timeline|Timeline_0 Play)
              (:Update
                (Transformation|SetRelativeTransform _saberblade (Math|Transform|MakeTransform (Math|Vector|MakeVector 0.0 0.0 _location) (.Rotation (Math|Transform|BreakTransform (Transformation|GetRelativeTransform _saberblade))) (Math|Vector|MakeVector 0.551969 0.551969 _size)) false false))
              (:event_start
                (if (Variables|Default|Getisforwarding)
                  (Variables|Default|Setissaberout true)
                  (Rendering|SetVisibility (Variables|Default|GetPointLight) true false)
                  (else
                    (Rendering|SetVisibility (Variables|Default|GetPointLight) false false))))
              (:event_end
                (if (not (Variables|Default|Getisforwarding))
                  (Variables|Default|Setissaberout false)))))
          (:B
            (Variables|Default|Setisforwarding false)
            (Timeline|Timeline_0 Reverse))))
      (:then_1
        ;[1 1 1] clears all structs so it doesn't memorize any locations it shouldn't from before
        (Utilities|Array|Clear (Variables|Default|GetStructArray))))))

(event Input|KeyboardEvents|SpaceBar
  (params (Key :type Key%20Structure))
  ;[1 1 1] Force jump
  (:Pressed
    (bind _output_get (Variables|Default|Setholdingspacebar true))
    (Character|Jump)
    (if (and _output_get (not (< (.Z (Math|Vector|BreakVector (Transformation|GetVelocity))) 0.0))) :!label _label
      (Physics|AddImpulse (Variables|Character|GetCharacterMovement) "0, 0,130.000000" true)
      (Utilities|FlowControl|Delay 0.2)
      (goto _label)))
  (:Released
    (Variables|Default|Setholdingspacebar false)))

(fn ConstructionScript
  (bind _returnvalue (Rendering|Material|CreateDynamicMaterialInstance "/Game/Assets/phong3_Inst.phong3_Inst" :!class /Script/Engine.KismetMaterialLibrary))
  (bind _output_get (Variables|Default|SetSaberMat _returnvalue))
  (Rendering|Material|SetMaterial (Variables|Default|Getsaberblade) 0 _output_get)
  (Utilities|Array|Resize (Variables|Default|GetStructArray) 3))

(fn EnableMouseLook
  (Variables|Default|SetMouseAxisValueMultiplier 1.0))

(fn DisableMouseLook
  (Variables|Default|SetMouseAxisValueMultiplier 0.0))